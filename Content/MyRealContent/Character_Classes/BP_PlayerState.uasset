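; Player state that stores the chosen character class (Archer, Mage or Warrior) for the lobby.
; Three Server-named events ask GameMode_Lobby to swap the class on the default-index player controller, not explicitly the owning one, then record it in PlayerClass.
; CopyProperties carries PlayerClass over to the new player state, with debug prints of the class name and network authority.
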(event `self.ReceiveCopyProperties`
  (params (NewPlayerState :type "PlayerState Object Reference"))
  (bind _asbp_player_state (cast `/Game/MyRealContent/Character_Classes/BP_PlayerState` NewPlayerState))
  (bind _output_get (set `/Game/MyRealContent/Character_Classes/BP_PlayerState.PlayerClass` (`self.PlayerClass`) _asbp_player_state))
  (`KismetSystemLibrary.PrintString` (`KismetSystemLibrary.GetClassDisplayName` _output_get))
  (`/Engine/EditorBlueprintResources/ActorMacros.Switch Has Authority`
    (:`Authority`
      (`KismetSystemLibrary.PrintString` "Auth"))
    (:`Remote`
      (`KismetSystemLibrary.PrintString` "Rem"))))

(event `Server_ChangeToArcher`
  (bind _asgame_mode_lobby (cast `/Game/MyRealContent/Maps/Lobby/GameMode_Lobby` (`GameplayStatics.GetGameMode`)))
  (`/Game/MyRealContent/Maps/Lobby/GameMode_Lobby.ChangePlayerClass` _asgame_mode_lobby (`self.GetPlayerController`) "/Game/MyRealContent/Character_Classes/Class_Archer/BP_ArcherClass.BP_ArcherClass_C")
  (bind _output_get (set `self.PlayerClass` "/Game/MyRealContent/Character_Classes/Class_Archer/BP_ArcherClass.BP_ArcherClass_C"))
  (`KismetSystemLibrary.PrintString` (`KismetSystemLibrary.GetClassDisplayName` _output_get)))

(event `Server_ChangeToMage`
  (bind _asgame_mode_lobby (cast `/Game/MyRealContent/Maps/Lobby/GameMode_Lobby` (`GameplayStatics.GetGameMode`)))
  (`/Game/MyRealContent/Maps/Lobby/GameMode_Lobby.ChangePlayerClass` _asgame_mode_lobby (`self.GetPlayerController`) "/Game/MyRealContent/Character_Classes/Class_Mage/BP_MageClass.BP_MageClass_C")
  (set `self.PlayerClass` "/Game/MyRealContent/Character_Classes/Class_Mage/BP_MageClass.BP_MageClass_C"))

(event `Server_ChangeToWarrior`
  (bind _asgame_mode_lobby (cast `/Game/MyRealContent/Maps/Lobby/GameMode_Lobby` (`GameplayStatics.GetGameMode`)))
  (`/Game/MyRealContent/Maps/Lobby/GameMode_Lobby.ChangePlayerClass` _asgame_mode_lobby (`self.GetPlayerController`) "/Game/MyRealContent/Character_Classes/Class_Warrior/BP_WarriorClass.BP_WarriorClass_C")
  (set `self.PlayerClass` "/Game/MyRealContent/Character_Classes/Class_Warrior/BP_WarriorClass.BP_WarriorClass_C"))

(fn `UserConstructionScript`)