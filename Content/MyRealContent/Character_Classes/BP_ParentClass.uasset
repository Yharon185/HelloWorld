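; Parent character Blueprint for a networked melee game, handling jumping, basic attacks, health, death and reset.
; Attacks route to the server, which multicasts the montage behind a short lockout; helper functions toggle damage on the child-actor weapon.
; Damage lowers clamped health, shown as debug text each tick.
; At zero health it disables input, multicasts a ragdoll and asks GameMode_Testing to reset the player after a delay.
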(event `self.ReceiveBeginPlay`
  (`/Engine/EditorBlueprintResources/ActorMacros.Switch Has Authority`
    (:`Authority`
      (`|ExecutionSequence`
        (:`then_0`
          (`self.SetOwner` (`ChildActorComponent.ChildActor` (`self.ChildActor`)) self))
        (:`then_1`
          (`self.Set Health` 2))))))

(event `self.ReceiveAnyDamage`
  (params (Damage :type "Float (single-precision)") (DamageType :type "DamageType Object Reference") (InstigatedBy :type "Controller Object Reference") (DamageCauser :type "Actor Object Reference"))
  (`self.DamageHealth` Damage))

(event `self.ReceiveTick`
  (params (DeltaSeconds :type "Float (single-precision)"))
  (`self.Debug Health` true))

(event `Client_DisableInput`
  (bind _returnvalue (`GameplayStatics.GetPlayerController` 0))
  ;[1 1 1] Death and Reset
  (`self.DisableInput` _returnvalue _returnvalue))

(event `self.CapsuleComponent.OnComponentBeginOverlap`
  (params (OverlappedComponent :type "PrimitiveComponent Object Reference") (OtherActor :type "Actor Object Reference") (OtherComp :type "PrimitiveComponent Object Reference") (OtherBodyIndex :type Integer) (bFromSweep :type Boolean) (SweepResult :type "HitResult Structure (by ref)")))

(event `AttackIfCan`
  (if (not (`self.Attacking`))
    (`self.MultiPlayerBasicAttack`)
    (set `self.Attacking` true)
    (`KismetSystemLibrary.Delay` 0.5)
    (set `self.Attacking` false)))

(event `Multi_Death`
  ;[1 1 1] Death and Reset
  (`PrimitiveComponent.SetCollisionEnabled` (`self.CapsuleComponent`) "QueryAndPhysics")
  (`PrimitiveComponent.SetCollisionEnabled` (`self.Mesh`) "QueryAndPhysics")
  (`SkeletalMeshComponent.SetAllBodiesSimulatePhysics` (`self.Mesh`) true))

(event `ServerPlayBasicAttack`
  (`self.AttackIfCan`))

(event `MultiPlayerBasicAttack`
  (`self.Play Basic Attack`))

(event `Cooldown From Hit`
  (`KismetSystemLibrary.Delay` 1.5)
  (set `self.DamageCooldown` false))

(event `Key|SpaceBar`
  (params (Key :type "Key Structure"))
  (bind _attacking (`self.Attacking`))
  (:`Pressed`
    (if (not _attacking)
      (`self.Jump`)))
  (:`Released`
    (if (not _attacking)
      (`self.StopJumping`))))

(event `ResetPlayerAfterTime`
  (params (Duration :type "Float (double-precision)" :default 2.0))
  (`KismetSystemLibrary.Delay` Duration)
  (`self.Reset Player`))

(fn `DamageHealth`
  (params (Damage :type "Float (double-precision)"))
  (if (`self.IsAlive`)
    (`self.Set Health` (- (`self.Health`) (`KismetMathLibrary.FTrunc` Damage)))
    (if (not (`self.IsAlive`))
      (`self.Client_DisableInput`)
      (`self.Multi_Death`)
      (`self.ResetPlayerAfterTime` 2.0))))

(fn `Debug Health`
  (params (Enabled :type Boolean :default true))
  (if Enabled
    (`KismetSystemLibrary.DrawDebugString` (+ (`self.GetActorEyesViewPoint`) (0.0 0.0 20.0)) (`KismetStringLibrary.Conv_IntToString` (`self.Health`)) null (struct :`R` 1.0 :`A` 1.0))))

(fn `DisableDamage`
  (bind _asbp_parent_weapon (cast `/Game/MyRealContent/Character_Classes/BP_ParentWeapon` (`ChildActorComponent.ChildActor` (`self.ChildActor`))))
  (`/Game/MyRealContent/Character_Classes/BP_ParentWeapon.DeActivateDamage` _asbp_parent_weapon))

(fn `EnableDamage`
  (bind _asbp_parent_weapon (cast `/Game/MyRealContent/Character_Classes/BP_ParentWeapon` (`ChildActorComponent.ChildActor` (`self.ChildActor`))))
  (`/Game/MyRealContent/Character_Classes/BP_ParentWeapon.Activate Damage` _asbp_parent_weapon))

(fn `GetHit`
  (`/Engine/EditorBlueprintResources/ActorMacros.Switch Has Authority`
    (:`Authority`
      (`self.DamageHealth` 1.0)
      (set `self.DamageCooldown` true)
      (`self.Cooldown From Hit`))))

(fn `IsAlive`
  (returns (ReturnValue :type Boolean))
  (return (> (`self.Health`) 0)))

(fn `Play Basic Attack`
  (`self.PlayAnimMontage` (`self.BasicAttack`)))

(fn `PlayJumpAnim`
  (params (AnimMontage :type "AnimMontage Object Reference"))
  (`self.PlayAnimMontage` AnimMontage))

(fn `Reset Player`
  (bind _asgame_mode_testing (cast `/Game/MyRealContent/GameModes/GameMode_Testing` (`GameplayStatics.GetGameMode`)))
  (bind _asplayer_controller (cast `PlayerController` (`self.GetController`)))
  (`/Game/MyRealContent/GameModes/GameMode_Testing.ResetPlayer` _asgame_mode_testing _asplayer_controller))

(fn `Set Health`
  (params (Health :type Integer))
  (set `self.Health` (`KismetMathLibrary.Clamp` Health 0 (`self.Max Health`))))

(fn `TryBasicAttack`
  (`/Engine/EditorBlueprintResources/ActorMacros.Switch Has Authority`
    (:`Authority`
      (`self.AttackIfCan`))
    (:`Remote`
      (`self.ServerPlayBasicAttack`))))

(fn `TryJump`
  (params (`Pressed/Released` :type Boolean))
  (if `Pressed/Released`
    (`self.Jump`)
    (else
      (`self.StopJumping`))))

(fn `UserConstructionScript`)