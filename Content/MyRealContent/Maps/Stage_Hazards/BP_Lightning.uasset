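; BP_Lightning is a short-lived stage hazard that, on the server, spawns BP_LightningExplosion at its transform and destroys itself after a brief delay.
; Box overlap chains ServerDamage, DealDamage and MultiDamage into ActivateDamage, meant to subtract Health from player pawn 0, not the overlapping actor.
; DealDamage requires LightningDamageCooldown true while ActivateDamage requires it false, and the delayed reset outlasts the actor's lifetime.
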(event `self.ReceiveBeginPlay`
  (`/Engine/EditorBlueprintResources/ActorMacros.Switch Has Authority`
    (:`Authority`
      (`KismetSystemLibrary.Delay` 0.1)
      (`|SpawnActorFromClass` "/Game/MyRealContent/Maps/Stage_Hazards/BP_LightningExplosion.BP_LightningExplosion_C" (`self.GetTransform`) "Undefined" "MultiplyWithRoot" null null)
      (`self.K2_DestroyActor`))))

(event `self.Box.OnComponentBeginOverlap`
  (params (OverlappedComponent :type "PrimitiveComponent Object Reference") (OtherActor :type "Actor Object Reference") (OtherComp :type "PrimitiveComponent Object Reference") (OtherBodyIndex :type Integer) (bFromSweep :type Boolean) (SweepResult :type "HitResult Structure (by ref)"))
  (`self.ServerDamage`)
  (set `self.LightningDamageCooldown` true))

(event `DealDamage`
  (if (`self.LightningDamageCooldown`)
    (`self.MultiDamage`)
    (`KismetSystemLibrary.Delay` 1.0)
    (set `self.LightningDamageCooldown` false)))

(event `ServerDamage`
  (`self.DealDamage`))

(event `MultiDamage`
  (`self.ActivateDamage`))

(fn `ActivateDamage`
  (locals (ParentClass :type "/Game/MyRealContent/Character_Classes/BP_ParentClass Object Reference"))
  (if (not (`self.LightningDamageCooldown`))
    (`/Engine/EditorBlueprintResources/ActorMacros.Switch Has Authority`
      (:`Authority`
        (bind _asbp_parent_class (cast `/Game/MyRealContent/Character_Classes/BP_ParentClass` (`GameplayStatics.GetPlayerPawn` 0)))
        (set `/Game/MyRealContent/Character_Classes/BP_ParentClass.Health` (- (`/Game/MyRealContent/Character_Classes/BP_ParentClass.Health` _asbp_parent_class) 1) _asbp_parent_class)))))

(fn `DeactivateDamage`
  (`/Engine/EditorBlueprintResources/ActorMacros.Switch Has Authority`
    (:`Authority`
      (set `self.LightningDamageCooldown` false))))

(fn `UserConstructionScript`)