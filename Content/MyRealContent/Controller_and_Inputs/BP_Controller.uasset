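; Player controller that routes Enhanced Input move, jump and basic attack actions to the possessed BP_ParentClass character.
; On replicated possession, the local controller caches the cast pawn and adds IMC_Controls.
; Input events call the character's functions, with movement forwarded only while it is not attacking.
; Helper functions add or remove mapping contexts, including a default controls, jump and attacks set that is not called here.
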(event `self.Pure_OnRepPosess`
  (params (PosessedPawn :type "Pawn Object Reference"))
  (if (`self.IsLocalPlayerController`)
    (bind _asbp_parent_class (cast `/Game/MyRealContent/Character_Classes/BP_ParentClass` PosessedPawn)
      (:`then`
        (set `self.As BP Parent Class` _asbp_parent_class)
        (`EnhancedInputSubsystemInterface.AddMappingContext` (subsystem `EnhancedInputLocalPlayerSubsystem`) "/Game/MyRealContent/Controller_and_Inputs/Inputs/IMC_Controls.IMC_Controls" 0 (struct)))
      (:`CastFailed`
        (`KismetSystemLibrary.PrintString` "Failed to cast")))))

(event `EnhancedInput|/Game/MyRealContent/Controller_and_Inputs/Inputs/IA_Move_Class`
  (params (ActionValue :type "Vector2D Structure") (ElapsedSeconds :type "Float (double-precision)") (TriggeredSeconds :type "Float (double-precision)") (InputAction :type "InputAction Object Reference" :default "/Game/MyRealContent/Controller_and_Inputs/Inputs/IA_Move_Class.IA_Move_Class"))
  (:`Triggered`
    (if (not (`/Game/MyRealContent/Character_Classes/BP_ParentClass.Attacking` (`self.As BP Parent Class`))) :!label _label
      (`MG_ParentClass.Pure_MoveCharacter` (`self.As BP Parent Class`) ActionValue)))
  (:`Canceled`
    (goto _label))
  (:`Completed`
    (goto _label)))

(event `EnhancedInput|/Game/MyRealContent/Controller_and_Inputs/Inputs/IA_BasicAttack`
  (params (ActionValue :type Boolean) (ElapsedSeconds :type "Float (double-precision)") (TriggeredSeconds :type "Float (double-precision)") (InputAction :type "InputAction Object Reference" :default "/Game/MyRealContent/Controller_and_Inputs/Inputs/IA_BasicAttack.IA_BasicAttack"))
  (:`Triggered`
    (`/Game/MyRealContent/Character_Classes/BP_ParentClass.Play Basic Attack` (`self.As BP Parent Class`))))

(event `EnhancedInput|/Game/MyRealContent/Controller_and_Inputs/Inputs/IA_Jump_Class`
  (params (ActionValue :type Boolean) (ElapsedSeconds :type "Float (double-precision)") (TriggeredSeconds :type "Float (double-precision)") (InputAction :type "InputAction Object Reference" :default "/Game/MyRealContent/Controller_and_Inputs/Inputs/IA_Jump_Class.IA_Jump_Class"))
  (:`Triggered`
    (`KismetSystemLibrary.PrintString` "Hello")
    (`/Game/MyRealContent/Character_Classes/BP_ParentClass.TryJump` (`self.As BP Parent Class`) ActionValue)))

(fn `Add Input`
  (params (MappingContext :type "InputMappingContext Object Reference") (Priority :type Integer) (`Options Ignore All Pressed Keys Until Release` :type Boolean :default true))
  (`EnhancedInputSubsystemInterface.AddMappingContext` (subsystem `EnhancedInputLocalPlayerSubsystem`) MappingContext 0 (struct)))

(fn `Remove Input`
  (params (MappingContext :type "InputMappingContext Object Reference"))
  (`EnhancedInputSubsystemInterface.RemoveMappingContext` (subsystem `EnhancedInputLocalPlayerSubsystem`) MappingContext (struct)))

(fn `Set Default Inputs`
  (for _array_element (`|MakeArray` "/Game/MyRealContent/Controller_and_Inputs/Inputs/IMC_Controls.IMC_Controls" "/Game/MyRealContent/Controller_and_Inputs/Inputs/IMC_Jump.IMC_Jump" "/Game/MyRealContent/Controller_and_Inputs/Inputs/IMC_Attacks.IMC_Attacks" :!type "InputMappingContext Object Reference")
    (`self.Add Input` _array_element 0 false)))

(fn `UserConstructionScript`)